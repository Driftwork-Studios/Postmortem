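; Bear trap actor that reacts when another actor overlaps it, currently a placeholder with no damage logic.
; The overlap event passes the other actor to TriggerTrap, then calls the parent overlap handler.
; TriggerTrap only prints a message naming that actor and noting the missing damage function.
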(event `self.ReceiveActorBeginOverlap`
  (params (OtherActor :type "Actor Object Reference"))
  (`self.TriggerTrap` OtherActor)
  (`parent.ReceiveActorBeginOverlap` OtherActor))

(event `self.TriggerTrap`
  (params (`Other Actor` :type "Actor Object Reference"))
  (`KismetSystemLibrary.PrintString` (`KismetTextLibrary.Conv_TextToString` (`|FormatText` "{Other Actor} has trigged a bear trap - currently missing a damage function" (`KismetSystemLibrary.GetDisplayName` `Other Actor`)))))

(fn `UserConstructionScript`
  (`parent.UserConstructionScript`))