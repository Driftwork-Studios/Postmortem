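; BP_BaseAI is a base AI actor with health and a helper for sorting perception stimuli.
; OnDamage subtracts damage from Health, prints the result and destroys the actor at zero or below.
; The ProcessStimuli macro filters sensed actors by the Player tag and routes to follow new actor, lost track of target, or ignore stimulus.
; No graph shown here calls the macro or handles movement.
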(event `/Game/FirstPerson/Blueprints/Interfaces/BPI_EnemyDamageInterface.OnDamage`
  (params (FloatDamage :type "Float (double-precision)"))
  (bind _output_get (set `self.Health` (- (`self.Health`) FloatDamage)))
  (`KismetSystemLibrary.PrintString` (`KismetStringLibrary.Conv_DoubleToString` _output_get))
  (if (<= _output_get 0.0)
    (`self.K2_DestroyActor`)))

(fn `UserConstructionScript`)