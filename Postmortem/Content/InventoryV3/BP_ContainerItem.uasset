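; BP_ContainerItem defines an inventory item that carries container rows, along with a name, icon, dimensions, actor to spawn and actions.
; Getter functions expose that data, including the rows held in ContainerRows.
; Rotate toggles IsRotated, which makes GetIcon return the rotated icon and GetDimensions swap X and Y.
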(fn `GetActions`
  (returns (Actions :type "Array of /Game/InventoryV3/Interaction/ContainerItemActions/E_ContainerItemAction Enum"))
  (return (`self.Actions`)))

(fn `GetActorToSpawn`
  (returns (ActorToSpawn :type "Actor Class Reference"))
  (return (`self.ActorToSpawn`)))

(fn `GetDimensions`
  (returns (Dimensions :type "IntPoint Structure"))
  (bind (_dimensions_x _dimensions_y) (break `IntPoint` (`self.Dimensions`)))
  (if (`self.IsRotated`)
    (return (make `IntPoint` _dimensions_y _dimensions_x))
    (else
      (return (`self.Dimensions`)))))

(fn `GetIcon`
  (returns (Icon :type "MaterialInterface Object Reference"))
  (if (`self.IsRotated`)
    (return (`self.IconRotated`))
    (else
      (return (`self.Icon`)))))

(fn `GetName`
  (returns (Name :type Text))
  (return (`self.Name`)))

(fn `GetRows`
  (returns (ContainerRows :type "Array of /Game/InventoryV3/S_ContainerRow Structure"))
  (return (`self.ContainerRows`)))

(fn `Rotate`
  (set `self.IsRotated` (not (`self.IsRotated`))))