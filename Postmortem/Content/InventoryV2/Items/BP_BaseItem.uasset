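; BP_BaseItem is a world pickup actor that gives its item to the player's inventory on overlap.
; On BeginPlay, if no ItemObject is set, it builds a BP_BaseItemObject from the DT_InventoryItemData row matching ItemID, copying dimensions, icons and item class.
; When a BP_PlayerCharacter enters the sphere, it calls TryAddItem on the inventory component and destroys itself only if that succeeds.
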(event `self.ReceiveBeginPlay`
  (if (not (`KismetSystemLibrary.IsValid` (`self.ItemObject`)))
    (bind _item_object (`self.GetDefaultItemObject`))
    (set `self.ItemObject` _item_object)))

(event `self.Sphere.OnComponentBeginOverlap`
  (params (OverlappedComponent :type "PrimitiveComponent Object Reference") (OtherActor :type "Actor Object Reference") (OtherComp :type "PrimitiveComponent Object Reference") (OtherBodyIndex :type Integer) (bFromSweep :type Boolean) (SweepResult :type "HitResult Structure (by ref)"))
  (bind _asbp_player_character (cast `/Game/FirstPerson/Blueprints/BP_PlayerCharacter` OtherActor))
  (bind _added (`/Game/InventoryV2/BPAC_InventoryComponent.TryAddItem` (`/Game/FirstPerson/Blueprints/BP_PlayerCharacter.BPAC_InventoryComponent` _asbp_player_character) (`self.ItemObject`)))
  (if _added
    (`self.K2_DestroyActor`)))

(fn `GetDefaultItemObject`
  (returns (`Item Object` :type "/Game/InventoryV2/Items/BP_BaseItemObject Object Reference"))
  (bind _itemid (`self.ItemID`))
  (bind _returnvalue (`|GetDataTableRow` "/Game/InventoryV2/DT_InventoryItemData.DT_InventoryItemData" (`KismetStringLibrary.Conv_StringToName` _itemid))
    (:`then`
      (bind (_itemname _itemcatagory _rarity _itemdescription _itemicon _itemiconrotated _itemclass _dimensions) (break `/Game/InventoryV2/S_ItemData` _returnvalue))
      (bind _returnvalue_2 (`|GenericCreateObject` self "/Game/InventoryV2/Items/BP_BaseItemObject.BP_BaseItemObject_C" (make `IntPoint` (break `IntPoint` _dimensions) (`.Y` (break `IntPoint` _dimensions))) _itemicon _itemiconrotated _itemclass))
      (return _returnvalue_2))
    (:`RowNotFound`
      (`KismetSystemLibrary.PrintText` (`|FormatText` "No row round for item with ItemID: \"{ItemID}\"" _itemid)))))

(fn `UserConstructionScript`)